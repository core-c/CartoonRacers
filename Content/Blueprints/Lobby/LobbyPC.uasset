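; LobbyPC is the player controller for the multiplayer lobby, owning each player's lobby menu and relaying their settings to the game mode.
; CallUpdate stores the player info, then has LobbyGM swap the cart and refresh everyone.
; Other events update the menu's player list, map and player count, or replace it with a loading screen.
; Being kicked opens the main menu and destroys the session, as does EndPlay; SaveGameCheck is empty.
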(event Custom|InitialSetup
  ;[1 1 1] Initial setup, check for savegame and call update
  (CallFunction|SaveGameCheck)
  (CallFunction|CallUpdate (Variables|PlayerInfo|GetPlayerSettings) false))

(event Custom|CallUpdate
  (params (Playerinfo :type Player%20Info%20Structure) (ChangedStatus :type Boolean))
  (bind _returnvalue (Game|GetGameMode))
  (bind _aslobby_gm (Utilities|Casting|CastToLobbyGM _returnvalue))
  ;[1 1 1] Assigns the selected team and cart and tells everyone to update the lobbymenu
  (Variables|PlayerInfo|SetPlayerSettings Playerinfo)
  (Default|SwapCharacter _aslobby_gm self (.PlayersCart (Utilities|Struct|BreakPlayerInfo (Variables|PlayerInfo|GetPlayerSettings))) ChangedStatus)
  (Default|EveryoneUpdate _aslobby_gm))

(event Custom|SetupLobbymenu
  (params (ServerName :type Text))
  ;[1 1 1] Setup and Display LobbyMenu
  (Variables|Default|SetbShowMouseCursor true)
  (bind _returnvalue (UserInterface|CreateWidget "/Game/UI/Lobby/LobbyMenu.LobbyMenu_C" self ServerName))
  (bind _output_get (Variables|Widgets|SetLobbyMenu_Ref _returnvalue))
  (UserInterface|Viewport|AddtoViewport _output_get 0)
  (Input|SetInputModeGameandUI self _output_get "DoNotLock" true))

(event Custom|AddPlayerinfo
  (params (Connected%20playersInfos :type Array%20of%20Player%20Info%20Structures))
  (bind _lobbymenu_ref (Variables|Widgets|GetLobbyMenu_Ref))
  ;[1 1 1] UpdatePlayerListWindow when called
  (Variables|Default|SetConnected%20Players%20Infos Connected%20playersInfos)
  (Utilities|IsValid _lobbymenu_ref
    (:Is%20Valid
      (Default|ClearPlayerList _lobbymenu_ref)
      (for _array_element (Variables|Default|GetConnected%20Players%20Infos)
        (Default|UpdatePlayerWindow (Variables|Widgets|GetLobbyMenu_Ref) _array_element)))))

(event Custom|UpdateLobbySettings
  (params (MapImage :type Texture%202D%20Object%20Reference) (MapName :type Text))
  (bind _lobbymenu_ref (Variables|Widgets|GetLobbyMenu_Ref))
  ;[1 1 1] Update LobbyInfo on the client
  (Variables|/Game/UI/Lobby/LobbyMenu.LobbyMenu_C|SetMapThumb _lobbymenu_ref MapImage)
  (Variables|/Game/UI/Lobby/LobbyMenu.LobbyMenu_C|SetMapName _lobbymenu_ref MapName))

(event Custom|ShowLoadingScreen
  ;[1 1 1] Remove LobbyMenu and show loading screen
  (Widget|RemovefromParent (Variables|Widgets|GetLobbyMenu_Ref))
  (bind _returnvalue (UserInterface|CreateWidget "/Game/UI/AllLevels/LoadingScreen.LoadingScreen_C" self))
  (UserInterface|Viewport|AddtoViewport _returnvalue 0))

(event Custom|UpdateNumberOfPlayers
  (params (CurrentPlayers :type Integer) (MaxPlayers :type Integer))
  (bind _lobbymenu_ref (Variables|Widgets|GetLobbyMenu_Ref))
  ;[1 1 1] Update the number of players
  (Utilities|IsValid _lobbymenu_ref
    (:Is%20Valid
      (Variables|/Game/UI/Lobby/LobbyMenu.LobbyMenu_C|SetPlayersDisplay _lobbymenu_ref (Utilities|Text|ToText(String) (Utilities|String|Append (Utilities|String|ToString(Integer) CurrentPlayers) " / " (Utilities|String|ToString(Integer) MaxPlayers)))))))

(event Custom|Kicked
  ;[1 1 1] Called when Server Disconnect or player is kicked
  (Game|OpenLevel(byName) "MainMenu")
  (|DestroySession self))

(event EventEndPlay
  (params (EndPlayReason :type EEndPlayReason%20Enum :default "Destroyed"))
  ;[1 1 1] Called when Server Disconnect or player is kicked
  (|DestroySession self))

(event Input|KeyboardEvents|T
  (params (Key :type Key%20Structure :default "None"))
  (:Pressed
    (Utilities|FlowControl|FlipFlop
      (:A
        (Widget|SetVisibility (Variables|Widgets|GetLobbyMenu_Ref) "Hidden"))
      (:B
        (Widget|SetVisibility (Variables|Widgets|GetLobbyMenu_Ref) "Visible")))))

(fn ConstructionScript)

(fn SaveGameCheck)