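; Start light actor that runs a timed red, yellow, green countdown before opening the way at the start of play.
; On BeginPlay a chain of Delays swaps lit and dark materials on separate slots of its static mesh.
; When green lights, the Blocker component is destroyed to clear the path, and the green light goes dark after a further delay.
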(event EventBeginPlay
  (bind _staticmesh (Variables|Default|GetStaticMesh))
  (Utilities|FlowControl|Delay 2.0)
  (Rendering|Material|SetMaterial (Variables|Default|GetStaticMesh) 3 "/Game/Models/RaceProps/Red_Lit.Red_Lit")
  (Utilities|FlowControl|Delay 2.0)
  (Rendering|Material|SetMaterial (Variables|Default|GetStaticMesh) 3 "/Game/Models/RaceProps/Red_Dark.Red_Dark")
  (Rendering|Material|SetMaterial (Variables|Default|GetStaticMesh) 2 "/Game/Models/RaceProps/Yellow_lit.Yellow_lit")
  (Utilities|FlowControl|Delay 2.0)
  (Rendering|Material|SetMaterial (Variables|Default|GetStaticMesh) 1 "/Game/Models/RaceProps/Green_Lit.Green_Lit")
  (Rendering|Material|SetMaterial _staticmesh 2 "/Game/Models/RaceProps/Yellow_dark.Yellow_dark")
  (Components|DestroyComponent (Variables|Default|Getblocker))
  (Utilities|FlowControl|Delay 1e+01)
  (Rendering|Material|SetMaterial _staticmesh 1 "/Game/Models/RaceProps/Green_dark.Green_dark"))

(event Collision|EventActorBeginOverlap
  (params (OtherActor :type Actor%20Object%20Reference)))

(event EventTick
  (params (DeltaSeconds :type Float%20%28single-precision%29)))

(fn ConstructionScript)