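; RacoonCart is a vehicle Blueprint whose engine-side logic here is limited to speed-driven audio.
; Each Tick calls the parent, reads the Mesh's linear physics velocity and sets the Audio component's pitch multiplier to that speed scaled by a small constant.
; BeginPlay and overlap events are disabled stubs, the construction script only calls its parent, and the VehicleMovement reference is unused.
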(event EventBeginPlay
  (|CallParentFunction) ; This node is disabled and will not be called.\nDrag off pins to build functionality.
)

(event Collision|EventActorBeginOverlap
  (params (OtherActor :type Actor%20Object%20Reference)))

(event EventTick
  (params (DeltaSeconds :type Float%20%28single-precision%29))
  (|CallParentFunction DeltaSeconds)
  (bind _returnvalue (Physics|GetPhysicsLinearVelocity (Variables|Character|GetMesh) "None"))
  (Audio|Components|Audio|SetPitchMultiplier (Variables|Default|GetAudio) (* (Math|Vector|VectorLength _returnvalue) 0.005)))

(fn ConstructionScript
  (|CallParentFunction))